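; Game mode Blueprint that handles saving and restoring the player's position through a single save slot.
; On BeginPlay it loads the slot and moves the player character to the stored transform, or creates and saves a new SaveSlot1 if none exists.
; Guardar writes the player's current transform into the existing slot.
; Cargar restarts the level via console command, so BeginPlay reapplies the saved transform.
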(event Custom|Guardar
  (bind _returnvalue (SaveGame|LoadGamefromSlot (Variables|Default|GetSlot%20Name%201)))
  (bind _assave_slot_1 (Utilities|Casting|CastToSaveSlot1 _returnvalue))
  (Variables|/Game/Videojuegos3D/Blueprints/SaveSlot1.SaveSlot1_C|SetPlayerTranform _assave_slot_1 (Transformation|GetActorTransform (Game|GetPlayerCharacter 0)))
  (SaveGame|SaveGametoSlot _assave_slot_1 (Variables|Default|GetSlot%20Name%201)))

(event Custom|Cargar
  (Development|ExecuteConsoleCommand "RestartLevel" 0))

(event EventBeginPlay
  (bind _returnvalue (SaveGame|DoesSaveGameExist (Variables|Default|GetSlot%20Name%201)))
  (if _returnvalue
    ;[1 1 1] Carga de memoria y asigancion de sus variables
    (bind _returnvalue_2 (SaveGame|LoadGamefromSlot (Variables|Default|GetSlot%20Name%201)))
    (bind _assave_slot_1 (Utilities|Casting|CastToSaveSlot1 _returnvalue_2))
    (Transformation|SetWorldTransform (Variables|/Script/Engine.Actor|GetRootComponent (Game|GetPlayerCharacter 0)) (Variables|/Game/Videojuegos3D/Blueprints/SaveSlot1.SaveSlot1_C|GetPlayerTranform _assave_slot_1) false false)
    (else
      ;[1 1 1] Crear y guardar memoria si es que no se encuentra una previa
      (bind _returnvalue_3 (SaveGame|CreateSaveGameObject "/Game/Videojuegos3D/Blueprints/SaveSlot1.SaveSlot1_C"))
      (SaveGame|SaveGametoSlot _returnvalue_3 (Variables|Default|GetSlot%20Name%201)))))

(event EventTick
  (params (DeltaSeconds :type Float%20%28single-precision%29)))

(fn ConstructionScript)