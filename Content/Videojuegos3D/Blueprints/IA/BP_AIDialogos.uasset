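; BP_AIDialogos is an AI dialogue Blueprint that shows prompt text and timed dialogue lines on a player's HUD.
; MostrarMensaje and LimpiarMensaje set and clear a single message through the HUD's SetMensaje.
; IniciarDialogo loops through the Dialogos array with a counter and a configurable Delay between lines.
; After the last line it waits briefly, resets the counter and clears the player's EnDialogo flag, leaving the HUD text in place.
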(event EventBeginPlay
  (|CallParentFunction) ; This node is disabled and will not be called.\nDrag off pins to build functionality.
)

(event Collision|EventActorBeginOverlap
  (params (OtherActor :type Actor%20Object%20Reference))
  (|CallParentFunction OtherActor) ; This node is disabled and will not be called.\nDrag off pins to build functionality.
)

(event EventTick
  (params (DeltaSeconds :type Float%20%28single-precision%29))
  (|CallParentFunction DeltaSeconds) ; This node is disabled and will not be called.\nDrag off pins to build functionality.
)

(event EventMostrarMensaje
  (params (Player :type Main%20Character%20BP%20Object%20Reference))
  (Default|SetMensaje (Variables|/Game/Videojuegos3D/Blueprints/MainCharacterBP.MainCharacterBP_C|GetHUD Player) (Variables|Dialogo|GetMensaje)))

(event EventLimpiarMensaje
  (params (Player :type Main%20Character%20BP%20Object%20Reference))
  (Default|SetMensaje (Variables|/Game/Videojuegos3D/Blueprints/MainCharacterBP.MainCharacterBP_C|GetHUD Player)))

(event EventIniciarDialogo
  (params (Player :type Main%20Character%20BP%20Object%20Reference))
  (if (> (Utilities|Array|Length (Variables|Dialogo|GetDialogos)) (Variables|Default|GetContador)) :!label _label
    (Default|SetMensaje (Variables|/Game/Videojuegos3D/Blueprints/MainCharacterBP.MainCharacterBP_C|GetHUD Player) (Utilities|Array|Get(acopy) (Variables|Dialogo|GetDialogos) (Variables|Default|GetContador)))
    (Utilities|FlowControl|Delay (Variables|Dialogo|GetDurationEntreLineas))
    (Variables|Default|SetContador (+ (Variables|Default|GetContador) 1))
    (goto _label)
    (else
      (Utilities|FlowControl|Delay 1.0)
      (Variables|Default|SetContador 0)
      (Variables|/Game/Videojuegos3D/Blueprints/MainCharacterBP.MainCharacterBP_C|SetEnDialogo Player false))))

(fn ConstructionScript
  (|CallParentFunction))