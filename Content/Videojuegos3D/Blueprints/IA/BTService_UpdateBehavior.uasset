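; Behavior tree service that picks the behavior state for BP_AIBase-controlled pawns and writes it to a Blackboard enum key.
; It caches the pawn on search start, then re-evaluates on every service tick while that reference is valid.
; The Interactuar Blackboard flag takes priority; otherwise the state depends on whether the pawn has a valid PatrullaControl patrol reference, with a default state when it does not.
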(event EventReceiveSearchStartAI
  (params (OwnerController :type AI%20Controller%20Object%20Reference) (ControlledPawn :type Pawn%20Object%20Reference))
  (bind _asbp_aibase (Utilities|Casting|CastToBP_AIBase ControlledPawn))
  (Variables|Default|SetBP_AIBase _asbp_aibase))

(event EventReceiveTickAI
  (params (OwnerController :type AI%20Controller%20Object%20Reference) (ControlledPawn :type Pawn%20Object%20Reference) (DeltaSeconds :type Float%20%28single-precision%29))
  (Variables|Default|GetBP_AIBase
    (:then
      (if (Class|BTFunctionLibrary|GetBlackboardValueasBool (Variables|Default|GetInteractuarKey))
        (Utilities|SetBehavior "NewEnumerator4")
        (else
          (Variables|/Game/Videojuegos3D/Blueprints/IA/BP_AIBase.BP_AIBase_C|GetPatrullaControl (Variables|Default|GetBP_AIBase)
            (:then
              (Utilities|SetBehavior "NewEnumerator1"))
            (:else
              (Utilities|SetBehavior "NewEnumerator0"))))))
    (:else)))