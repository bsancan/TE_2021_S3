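; Base pickup-area actor for items that shows a HUD message while the main character stands in range.
; On Box overlap it caches the MainCharacterBP and its HUD, registers itself as that character's current Item and displays its Mensaje.
; Leaving the box clears the character's Item reference and blanks the message.
; MostarDosNombres is a stub returning an empty string, and the file holds no interaction logic itself.
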(event OnComponentBeginOverlap(Box)
  (params (OverlappedComponent :type Primitive%20Component%20Object%20Reference) (OtherActor :type Actor%20Object%20Reference) (OtherComp :type Primitive%20Component%20Object%20Reference) (OtherBodyIndex :type Integer) (bFromSweep :type Boolean) (SweepResult :type Hit%20Result%20Structure%20%28by%20ref%29))
  (bind _asmain_character_bp (Utilities|Casting|CastToMainCharacterBP OtherActor))
  (Variables|Default|SetMainCharacterRef _asmain_character_bp)
  (Variables|Default|SetHUD (Variables|/Game/Videojuegos3D/Blueprints/MainCharacterBP.MainCharacterBP_C|GetHUD _asmain_character_bp))
  (Variables|/Game/Videojuegos3D/Blueprints/MainCharacterBP.MainCharacterBP_C|SetItem _asmain_character_bp self)
  (CallFunction|MostrarMensajeInicial))

(event OnComponentEndOverlap(Box)
  (params (OverlappedComponent :type Primitive%20Component%20Object%20Reference) (OtherActor :type Actor%20Object%20Reference) (OtherComp :type Primitive%20Component%20Object%20Reference) (OtherBodyIndex :type Integer))
  (bind _asmain_character_bp (Utilities|Casting|CastToMainCharacterBP OtherActor))
  (Variables|Default|SetMainCharacterRef 0)
  (Variables|/Game/Videojuegos3D/Blueprints/MainCharacterBP.MainCharacterBP_C|SetItem _asmain_character_bp 0)
  (CallFunction|LimpiarMensaje))

(event EventBeginPlay)

(event Collision|EventActorBeginOverlap
  (params (OtherActor :type Actor%20Object%20Reference)))

(event EventTick
  (params (DeltaSeconds :type Float%20%28single-precision%29)))

(fn ConstructionScript)

(fn MostrarMensajeInicial
  (Default|SetMensaje (Variables|Default|GetHUD) (Variables|Item|GetMensaje)))

(fn LimpiarMensaje
  (Utilities|IsValid (Variables|Default|GetHUD)
    (:Is%20Valid
      (Default|SetMensaje (Variables|Default|GetHUD))
      (Variables|Default|SetHUD 0))))

(fn MostarDosNombres
  (params (Nombre :type String))
  (return ""))