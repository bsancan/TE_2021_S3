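; ItemVidas is a collectible item Blueprint that grants the main character extra lives.
; Its RecolectarItem event adds Cantidad to the character's Vidas and pushes the new total to the HUD.
; It then flashes a Spanish notification of the lives gained, calls LimpiarMensaje and destroys itself.
; Overlap and Tick are disabled stubs, so this graph only defines the collection effect.
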(event Collision|EventActorBeginOverlap
  (params (OtherActor :type Actor%20Object%20Reference))
  (|CallParentFunction OtherActor) ; This node is disabled and will not be called.\nDrag off pins to build functionality.
)

(event EventTick
  (params (DeltaSeconds :type Float%20%28single-precision%29))
  (|CallParentFunction DeltaSeconds) ; This node is disabled and will not be called.\nDrag off pins to build functionality.
)

(event EventRecolectarItem
  (bind _maincharacterref (Variables|Default|GetMainCharacterRef))
  (bind _hud (Variables|Default|GetHUD))
  (bind _output_get (Variables|/Game/Videojuegos3D/Blueprints/MainCharacterBP.MainCharacterBP_C|SetVidas _maincharacterref (+ (Variables|/Game/Videojuegos3D/Blueprints/MainCharacterBP.MainCharacterBP_C|GetVidas _maincharacterref) (Variables|Default|GetCantidad))))
  (Default|SetVidas _hud _output_get)
  (Default|NotificacionFlash _hud (Utilities|String|Append "Has ganado +" (Utilities|String|ToString(Integer) (Variables|Default|GetCantidad)) " vidas"))
  (CallFunction|LimpiarMensaje)
  (Actor|DestroyActor))

(fn ConstructionScript
  (|CallParentFunction))