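; ItemEspada is a sword pickup that equips the player character when collected.
; On RecolectarItem it spawns an Espada actor owned by the main character and snaps it to a back or waist socket on the character mesh, chosen by IrEnEspalda, which also sets the spawn rotation.
; It then sends its item message to the HUD, calls LimpiarMensaje and destroys itself.
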(event EventBeginPlay
  (|CallParentFunction) ; This node is disabled and will not be called.\nDrag off pins to build functionality.
)

(event Collision|EventActorBeginOverlap
  (params (OtherActor :type Actor%20Object%20Reference))
  (|CallParentFunction OtherActor) ; This node is disabled and will not be called.\nDrag off pins to build functionality.
)

(event EventTick
  (params (DeltaSeconds :type Float%20%28single-precision%29))
  (|CallParentFunction DeltaSeconds) ; This node is disabled and will not be called.\nDrag off pins to build functionality.
)

(event EventRecolectarItem
  (bind _returnvalue (Game|SpawnActorfromClass "/Game/Videojuegos3D/Blueprints/Items/Espada.Espada_C" (select (Variables|Item|GetIrEnEspalda) (Math|Transform|MakeTransform "0, 0, 0" "0.000000,90.000000, 0") (Math|Transform|MakeTransform "0, 0, 0" "0.000000,0.000000, 0")) "AdjustIfPossibleButAlwaysSpawn" (Variables|Default|GetMainCharacterRef) 0))
  (Transformation|AttachComponentToComponent _returnvalue (Variables|/Script/Engine.Character|GetMesh (Variables|Default|GetMainCharacterRef)) (select (Variables|Item|GetIrEnEspalda) (Variables|Default|GetEspaldaSocket) (Variables|Default|GetCinturaSocket)) "SnapToTarget" "KeepWorld" "KeepWorld" true)
  (Default|SetItem (Variables|Default|GetHUD) (Variables|Item|GetMensajeItem))
  (CallFunction|LimpiarMensaje)
  (Actor|DestroyActor))

(fn ConstructionScript
  (|CallParentFunction))